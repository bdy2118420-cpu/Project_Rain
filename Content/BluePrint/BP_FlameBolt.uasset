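; BP_FlameBolt is a flame bolt actor, apparently a projectile, that plays a Niagara impact effect where it hits.
; A collision component hit passes the impact location through C2S_Bomb to S2C_Bomb, a client-to-server-to-client relay by naming, which spawns the hit system there.
; OnActivated and OnDeactivated switch the bolt's own Niagara effect on and off.
; The graph contains no damage or destroy logic.
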(event `C2S_Bomb`
  (params (Location :type "Vector Structure"))
  (`self.S2C_Bomb` Location))

(event `self.CollisionComponent.OnComponentHit`
  (params (HitComponent :type "PrimitiveComponent Object Reference") (OtherActor :type "Actor Object Reference") (OtherComp :type "PrimitiveComponent Object Reference") (NormalImpulse :type "Vector Structure") (Hit :type "HitResult Structure (by ref)"))
  (`self.C2S_Bomb` (`.Location` (`GameplayStatics.BreakHitResult` Hit))))

(event `S2C_Bomb`
  (params (Location :type "Vector Structure"))
  (`NiagaraFunctionLibrary.SpawnSystemAtLocation` "/Game/Asset/FBX/NS_FlameBolt_Hit.NS_FlameBolt_Hit" Location))

(event `self.ReceiveOnActivated`
  (`ActorComponent.Activate` (`self.NS_FlameBolt`) true))

(event `self.ReceiveOnDeactivated`
  (`ActorComponent.Deactivate` (`self.NS_FlameBolt`)))

(fn `UserConstructionScript`)