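; Ranged monster Blueprint that handles health UI, damage feedback and death.
; BeginPlay binds the health component to an HP bar widget, and each health change sends the difference from the previous value to the first player's mage controller as floating damage text.
; Death relays through client-to-server and server-to-client events (by naming), which disable capsule collision, ragdoll the mesh, stop AI logic and deactivate the monster after a short delay.
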(event `self.ReceiveBeginPlay`
  (set `self.PreviousHealth` (`HealthComponent.MaxHealth` (`self.HealthComp`)))
  (bind _aswbp_hpbar (cast `/Game/UI/WBP_HPBar` (`WidgetComponent.GetUserWidgetObject` (`self.Widget`))))
  (set `/Game/UI/WBP_HPBar.TargetHealth` (`self.HealthComp`) _aswbp_hpbar))

(event `self.HealthComp.OnHealthChanged`
  (params (HealthComp :type "HealthComponent Object Reference") (Health :type "Float (single-precision)") (MaxHealth :type "Float (single-precision)"))
  (set `self.Damage` (- (`self.PreviousHealth`) Health))
  (set `self.PreviousHealth` Health)
  (bind _asbp_mage_controller (cast `/Game/BluePrint/FieldCore/BP_MageController` (`GameplayStatics.GetPlayerController` 0)))
  (`/Game/BluePrint/FieldCore/BP_MageController.Show DamageText` _asbp_mage_controller (`KismetMathLibrary.Conv_IntToDouble` (`KismetMathLibrary.FTrunc` (`self.Damage`))) (`self.K2_GetActorLocation`)))

(event `self.HealthComp.OnDeath`
  (params (DeadActor :type "Actor Object Reference"))
  (`self.C2S_Death`))

(event `C2S_Death`
  (`self.S2C_Death`))

(event `S2C_Death`
  (bind _mesh (`self.Mesh`))
  (`PrimitiveComponent.SetCollisionEnabled` (`self.CapsuleComponent`) "NoCollision")
  (`PrimitiveComponent.SetCollisionProfileName` _mesh "Ragdoll" true)
  (`PrimitiveComponent.SetSimulatePhysics` _mesh true)
  (bind _asmonster_aicontroller (cast `MonsterAIController` (`self.GetController`)))
  (`BrainComponent.StopLogic` (`AIController.BrainComponent` _asmonster_aicontroller) "")
  (`KismetSystemLibrary.Delay` 2.0)
  (`self.DeactivateMonster`))

(fn `UserConstructionScript`)