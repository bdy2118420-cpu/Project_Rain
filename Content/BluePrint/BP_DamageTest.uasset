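; BP_DamageTest is a damage test actor that shows the damage it takes as text.
; On each Health change event it derives damage from the difference to the stored previous health, then updates that stored value.
; It passes the truncated amount and its own location to ShowDamageText on player 0's BP_MageController.
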(event `self.Health.OnHealthChanged`
  (params (HealthComp :type "HealthComponent Object Reference") (Health :type "Float (single-precision)") (MaxHealth :type "Float (single-precision)"))
  (set `self.Damage` (- (`self.PreviousHealth`) Health))
  (set `self.PreviousHealth` Health)
  (bind _asbp_mage_controller (cast `/Game/BluePrint/FieldCore/BP_MageController` (`GameplayStatics.GetPlayerController` 0)))
  (`/Game/BluePrint/FieldCore/BP_MageController.Show DamageText` _asbp_mage_controller (`KismetMathLibrary.Conv_IntToDouble` (`KismetMathLibrary.FTrunc` (`self.Damage`))) (`self.K2_GetActorLocation`)))

(fn `UserConstructionScript`)