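; Player controller for the mage that sets up local input and HUD and displays floating damage numbers.
; On BeginPlay, the local controller adds the IMC_Mage mapping context, creates WBP_Main and pre-spawns a hidden pool of BP_DamageTextActor instances.
; ShowDamageText reuses the first hidden pooled actor, moves it above the hit with random horizontal jitter, sets the amount on its widget and calls PopUpActor.
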(event `self.ReceiveBeginPlay`
  (if (`self.IsLocalPlayerController`)
    (`EnhancedInputSubsystemInterface.AddMappingContext` (pcsubsystem `EnhancedInputLocalPlayerSubsystem` self) "/Game/Input/IMC_Mage.IMC_Mage" 0 (struct))
    (bind _returnvalue (`|CreateWidget` "/Game/UI/WBP_Main.WBP_Main_C"))
    (`UserWidget.AddToViewport` _returnvalue 0)
    (for _ (range 1 31)
      (bind _returnvalue_2 (`|SpawnActorFromClass` "/Game/BluePrint/UI/BP_DamageTextActor.BP_DamageTextActor_C" (`KismetMathLibrary.MakeTransform` (0.0 0.0 0.0)) "Undefined" "MultiplyWithRoot" null null))
      (`self.SetActorHiddenInGame` _returnvalue_2 true)
      (`KismetArrayLibrary.Array_Add` (`self.DamagePool`) _returnvalue_2))))

(fn `Show DamageText`
  (params (DamageAmount :type "Float (double-precision)") (HitLocation :type "Vector Structure"))
  (for _array_element (`self.DamagePool`)
    (if (`Actor.bHidden` _array_element)
      (`self.SetActorHiddenInGame` _array_element false)
      (`self.K2_SetActorLocation` _array_element (+ HitLocation (`KismetMathLibrary.MakeVector` (`KismetMathLibrary.RandomFloatInRange` -40.0 40.0) (`KismetMathLibrary.RandomFloatInRange` -40.0 40.0) 50.0)) false false)
      (bind _aswbp_damage_text (cast `/Game/UI/WBP_DamageText` (`WidgetComponent.GetUserWidgetObject` (`/Game/BluePrint/UI/BP_DamageTextActor.Widget` _array_element))))
      (`/Game/UI/WBP_DamageText.InitDamageText` _aswbp_damage_text (`local.DamageAmount`))
      (`/Game/BluePrint/UI/BP_DamageTextActor.PopUpActor` _array_element)
      (break))))

(fn `UserConstructionScript`)