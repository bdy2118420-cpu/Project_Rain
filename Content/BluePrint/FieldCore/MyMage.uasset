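; MyMage is a mage character Blueprint that handles damage feedback and death through its health component.
; It derives damage from the change in health and has the first player's BP_MageController show it as truncated floating text at the mage's location.
; Death passes through client-to-server and server-to-client named events, then disables player-0 input and capsule collision and ragdolls the mesh.
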(event `self.ReceiveBeginPlay`
  (set `self.PreviousHealth` (`HealthComponent.MaxHealth` (`self.HealthComp`))))

(event `self.HealthComp.OnHealthChanged`
  (params (HealthComp :type "HealthComponent Object Reference") (Health :type "Float (single-precision)") (MaxHealth :type "Float (single-precision)"))
  (set `self.Damage` (- (`self.PreviousHealth`) Health))
  (set `self.PreviousHealth` Health)
  (bind _asbp_mage_controller (cast `/Game/BluePrint/FieldCore/BP_MageController` (`GameplayStatics.GetPlayerController` 0)))
  (`/Game/BluePrint/FieldCore/BP_MageController.Show DamageText` _asbp_mage_controller (`KismetMathLibrary.Conv_IntToDouble` (`KismetMathLibrary.FTrunc` (`self.Damage`))) (`self.K2_GetActorLocation`)))

(event `self.HealthComp.OnDeath`
  (params (DeadActor :type "Actor Object Reference"))
  (`self.C2S_Death`))

(event `C2S_Death`
  (`self.S2C_Death`))

(event `S2C_Death`
  (bind _mesh (`self.Mesh`))
  (`self.DisableInput` (`GameplayStatics.GetPlayerController` 0))
  (`PrimitiveComponent.SetCollisionEnabled` (`self.CapsuleComponent`) "NoCollision")
  (`PrimitiveComponent.SetCollisionProfileName` _mesh "Ragdoll" true)
  (`PrimitiveComponent.SetSimulatePhysics` _mesh true))

(fn `UserConstructionScript`)